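; BP_Kreissegment is a circle-segment actor with a pie chart component and a cube, apparently a test for detecting overlap with a hand.
; Begin-overlap events on both components print the name of their own overlapped component.
; The OverplappHand event takes a Hand but only prints whether collision is enabled on the pie chart.
; All logic is debug output, and a direct Hand overlap check is left unconnected.
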(event `self.ReceiveActorBeginOverlap`
  (params (OtherActor :type "Actor Object Reference")))

(event `OverplappHand`
  (params (Hand :type "PrimitiveComponent Object Reference"))
  (`KismetSystemLibrary.PrintString` (`KismetStringLibrary.Conv_BoolToString` (`PrimitiveComponent.K2_IsCollisionEnabled` (`self.Pie_Chart`)))))

(event `self.Pie_Chart.OnComponentBeginOverlap`
  (params (OverlappedComponent :type "PrimitiveComponent Object Reference") (OtherActor :type "Actor Object Reference") (OtherComp :type "PrimitiveComponent Object Reference") (OtherBodyIndex :type Integer) (bFromSweep :type Boolean) (SweepResult :type "HitResult Structure (by ref)"))
  (`KismetSystemLibrary.PrintString` (`KismetSystemLibrary.GetDisplayName` OverlappedComponent)))

(event `self.Cube.OnComponentBeginOverlap`
  (params (OverlappedComponent :type "PrimitiveComponent Object Reference") (OtherActor :type "Actor Object Reference") (OtherComp :type "PrimitiveComponent Object Reference") (OtherBodyIndex :type Integer) (bFromSweep :type Boolean) (SweepResult :type "HitResult Structure (by ref)"))
  (`KismetSystemLibrary.PrintString` (`KismetSystemLibrary.GetDisplayName` OverlappedComponent)))

(fn `UserConstructionScript`)