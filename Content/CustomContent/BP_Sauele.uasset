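; BP_Sauele is a column actor that visualizes a party's election result as a bar height.
; SetYearHeight reads the Wahlergebnisse2 data table row for Partyname and scales Z for 2005, 2009 or 2013, starting at 2013.
; Box overlaps or SetStates toggle IsActiv; if the player still overlaps after a retriggerable delay, the column becomes a donor.
; Tick swaps between default, active and donor materials to show the current state.
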(event `self.ReceiveBeginPlay`
  (set `self.BoxMesh` (`self.StaticMeshComponent`))
  (`self.SetYearHeight` 2013))

(event `SetYearHeight`
  (params (Year :type Integer))
  ;[1 1 1] Höhe der Saeulen aus Tabelle setzen
  (bind _returnvalue (`|GetDataTableRow` "/Game/CustomContent/wahlergebnisse2.wahlergebnisse2" (`KismetStringLibrary.Conv_StringToName` (`self.partyname`)))
    (:`then`
      (switch `string` (`KismetStringLibrary.Conv_IntToString` Year)
        (:`2013`
          ;;[1 1 1] 2013
          (`self.SetActorScale3D` (`KismetMathLibrary.MakeVector` (.x (`self.GetActorScale3D`)) (.y (`self.GetActorScale3D`)) (* (`.2013_33_11F96DCC4FE060B9AAAFFEA740BF2AF4` (break `/Game/CustomContent/ParteiData` _returnvalue)) 0.4))))
        (:`2009`
          ;;[1 1 1] 2009
          (`self.SetActorScale3D` (`KismetMathLibrary.MakeVector` (.x (`self.GetActorScale3D`)) (.y (`self.GetActorScale3D`)) (* (`.2009_34_1A400C95484274407D390498C13AA1EB` (break `/Game/CustomContent/ParteiData` _returnvalue)) 0.4))))
        (:`2005`
          ;;[1 1 1] 2005
          (`self.SetActorScale3D` (`KismetMathLibrary.MakeVector` (.x (`self.GetActorScale3D`)) (.y (`self.GetActorScale3D`)) (* (`.2005_35_9C9C34774585DE5F8FAA2F8F3BEADDF3` (break `/Game/CustomContent/ParteiData` _returnvalue)) 0.4))))))))

(event `self.Box.OnComponentBeginOverlap`
  (params (OverlappedComponent :type "PrimitiveComponent Object Reference") (OtherActor :type "Actor Object Reference") (OtherComp :type "PrimitiveComponent Object Reference") (OtherBodyIndex :type Integer) (bFromSweep :type Boolean) (SweepResult :type "HitResult Structure (by ref)"))
  ;[0.14 0.14 0.14] Logik zum Setzen der States beim Überlappen
  ;;[1 1 1] wenn isActive true --> false & false --> true
  (set `self.isActiv` (not (`self.isActiv`)) :!label _label)
  (if (`self.isActiv`)
    (`KismetSystemLibrary.RetriggerableDelay` 1.0)
    (if (`self.IsOverlappingActor` (`GameplayStatics.GetPlayerPawn` 0))
      (set `self.isDonor` true)
      (set `self.activatedDonor` true))
    (else
      (set `self.isDonor` false))))

(event `SetStates`
  ;[0.14 0.14 0.14] Logik zum Setzen der States beim Überlappen
  (goto _label))

(event `ChangeDonorState`
  (params (isDonor :type Boolean))
  ;[1 1 1] Funktionen zum Aktualisieren der aktuellen Zustände
  (set `self.isDonor` isDonor))

(event `ChangedActivatedDonor`
  (params (isActivatedDonor :type Boolean))
  ;[1 1 1] Funktionen zum Aktualisieren der aktuellen Zustände
  (set `self.activatedDonor` isActivatedDonor))

(event `self.ReceiveTick`
  (params (DeltaSeconds :type "Float (single-precision)"))
  ;[1 1 1] Logik zum Einfärben der Säulen
  (if (`self.isActiv`)
    (`PrimitiveComponent.SetMaterial` (`self.StaticMeshComponent`) 0 "/Game/CustomContent/Material/M_Active.M_Active")
    (if (`self.isDonor`)
      (`PrimitiveComponent.SetMaterial` (`self.StaticMeshComponent`) 0 "/Game/CustomContent/Material/M_Donor.M_Donor"))
    (else
      (`PrimitiveComponent.SetMaterial` (`self.StaticMeshComponent`) 0 (`self.defaultMaterial`)))))

(fn `SetActive`
  (set `self.isActiv` true))

(fn `UserConstructionScript`)